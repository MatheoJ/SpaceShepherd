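; Planet actor that serves as a radial gravity source, supplying pull direction and strength for a given actor.
; Construction sizes the surface and falloff spheres from their radii and rebuilds a single PlanetMesh instance scaled to the surface radius.
; Gravity direction points toward the planet's center.
; Gravity scale is the inverse square of squared distance normalized between both spheres, so it grows unbounded approaching the surface and equals one at the falloff edge.
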(fn `GetGravityDirection`
  (params (Actor :type "Actor Object Reference"))
  (returns (GravityDirection :type "Vector Structure"))
  (return (`KismetMathLibrary.GetDirectionUnitVector` (`self.K2_GetActorLocation` Actor) (`self.K2_GetActorLocation`))))

(fn `GetGravityScale`
  (params (Actor :type "Actor Object Reference"))
  (returns (GravityScale :type "Float (double-precision)"))
  (return (/ 1.0 (`KismetMathLibrary.Square` (`KismetMathLibrary.NormalizeToRange` (`KismetMathLibrary.Vector_DistanceSquared` (`self.K2_GetActorLocation`) (`self.K2_GetActorLocation` Actor)) (`KismetMathLibrary.Square` (`SphereComponent.GetScaledSphereRadius` (`self.SurfaceSphere`))) (`KismetMathLibrary.Square` (`SphereComponent.GetScaledSphereRadius` (`self.FalloffSphere`))))))))

(fn `UserConstructionScript`
  (bind _planetmesh (`self.PlanetMesh`))
  (`parent.UserConstructionScript`)
  (`SphereComponent.SetSphereRadius` (`self.SurfaceSphere`) (`self.SurfaceRadius`) true)
  (`SphereComponent.SetSphereRadius` (`self.FalloffSphere`) (`self.FalloffRadius`) true)
  (`InstancedStaticMeshComponent.ClearInstances` _planetmesh)
  (`InstancedStaticMeshComponent.AddInstance` _planetmesh (`KismetMathLibrary.MakeTransform` (`self.K2_GetActorLocation`) (struct) (`KismetMathLibrary.Conv_DoubleToVector` (/ (`self.SurfaceRadius`) 100.0))) true))