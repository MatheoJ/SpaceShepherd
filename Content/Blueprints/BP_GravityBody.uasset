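; BP_GravityBody is a gravity source actor that sets a character's gravity direction and strength.
; ApplyGravity writes GetGravityDirection and GetGravityScale, multiplied by the Gravity variable, to the CharacterMovement component, and prints the resulting scale.
; Both getters return zero here, apparently as placeholders for child classes to override.
; The construction script locks actor scale to one, leaving size to a radius property.
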(fn `ApplyGravity`
  (params (Character :type "Character Object Reference"))
  (bind _charactermovement (`Character.CharacterMovement` Character))
  (bind _returnvalue (* (`self.GetGravityScale` Character) (`self.Gravity`)))
  (`CharacterMovementComponent.SetGravityDirection` _charactermovement (`self.GetGravityDirection` Character))
  (set `CharacterMovementComponent.GravityScale` _returnvalue _charactermovement)
  (`KismetSystemLibrary.PrintString` (`KismetStringLibrary.Conv_DoubleToString` _returnvalue)))

(fn `GetGravityDirection`
  (params (Actor :type "Actor Object Reference"))
  (returns (GravityDirection :type "Vector Structure"))
  (return (0.0 0.0 0.0)))

(fn `GetGravityScale`
  (params (Actor :type "Actor Object Reference"))
  (returns (GravityScale :type "Float (double-precision)"))
  (return 0.0))

(fn `UserConstructionScript`
  (`self.SetActorScale3D` (1.0 1.0 1.0)) ; Prevent changing scale, size is handled by radius property
)