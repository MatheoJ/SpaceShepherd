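; Actor component that applies planetary gravity to the Character that owns it.
; Body influence enter and exit events set or clear the current BP_GravityBody, and any body's exit clears it even if another is current.
; Each tick, at a custom interval, it delegates to that body's ApplyGravity, passing the character.
; On a non-Character owner it raises a script error instead.
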(event `On Enter Body Influence`
  (params (Body :type "Object Object Reference"))
  (bind _asbp_gravity_body (cast `/Game/Blueprints/Planets/BP_GravityBody` Body))
  (set `self.CurrentGravityBody` _asbp_gravity_body))

(event `On Exit Body Influence`
  (params (Body :type "Object Object Reference"))
  (cast `/Game/Blueprints/Planets/BP_GravityBody` Body)
  (set `self.CurrentGravityBody` null))

(event `self.ReceiveTick`
  (params (DeltaSeconds :type "Float (single-precision)"))
  (bind _currentgravitybody (`self.CurrentGravityBody`))
  (bind _ascharacter (cast `Character` (`self.GetOwner`))
    (:`then`
      (`/Engine/EditorBlueprintResources/StandardMacros.IsValid` _currentgravitybody
        (:`Is Valid`
          (`/Game/Blueprints/Planets/BP_GravityBody.ApplyGravity` _currentgravitybody _ascharacter))))
    (:`CastFailed`
      (`KismetSystemLibrary.RaiseScriptError` "A non-character actor has a GravityUpdater component. It will do nothing."))))