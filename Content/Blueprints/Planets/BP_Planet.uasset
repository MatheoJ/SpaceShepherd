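; BP_Planet is a spherical planet that supplies point gravity toward its center for any given actor.
; Its construction script sizes the surface and falloff spheres, rebuilds a single scaled mesh instance and scales the atmosphere to the falloff radius.
; Query functions return the unit direction to the center and a gravity scale, computed from a radius-based falloff times Gravity, normalized to Earth gravity.
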(fn `GetGravityDirection`
  (params (Actor :type "Actor Object Reference"))
  (returns (GravityDirection :type "Vector Structure"))
  (return (`KismetMathLibrary.GetDirectionUnitVector` (`self.K2_GetActorLocation` Actor) (`self.K2_GetActorLocation`))))

(fn `GetGravityScale`
  (params (Actor :type "Actor Object Reference"))
  (returns (GravityScale :type "Float (double-precision)"))
  (bind _returnvalue (`PlanetFunctionLibrary.GravityFalloff` (`self.K2_GetActorLocation` Actor) (`self.K2_GetActorLocation`) (`self.SurfaceRadius`) (`self.FalloffRadius`)))
  (return (/ (* _returnvalue (`self.Gravity`)) 9.81)))

(fn `UserConstructionScript`
  (bind _planetmesh (`self.PlanetMesh`))
  (`parent.UserConstructionScript`)
  (`SphereComponent.SetSphereRadius` (`self.SurfaceSphere`) (`self.SurfaceRadius`) true)
  (`SphereComponent.SetSphereRadius` (`self.FalloffSphere`) (`self.FalloffRadius`) true)
  (`InstancedStaticMeshComponent.ClearInstances` _planetmesh)
  (`InstancedStaticMeshComponent.AddInstance` _planetmesh (`KismetMathLibrary.MakeTransform` (`self.K2_GetActorLocation`) (struct) (`KismetMathLibrary.Conv_DoubleToVector` (/ (`self.SurfaceRadius`) 100.0))) true)
  (`SceneComponent.SetWorldScale3D` (`self.Atmosphere`) (`KismetMathLibrary.Conv_DoubleToVector` (/ (* (`self.FalloffRadius`) 2.0) 1000.0))))